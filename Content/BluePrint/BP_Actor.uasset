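; Spline-based actor that can place repeated static mesh components along its Spline.
; CreatMesh divides the spline length by a fixed Distance and adds an unrotated, unit-scale mesh at each interval in local space.
; The construction script is empty apart from disconnected leftovers of similar logic, the event graph is unused, and nothing in these graphs calls CreatMesh.
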(fn `CreatMesh`
  (bind _distance (`self.Distance`))
  (set `self.Distance` 5.0)
  (for _index (range (+ (`KismetMathLibrary.FTrunc` (/ (`SplineComponent.GetSplineLength` (`self.Spline`)) _distance)) 1))
    (`AddComponent|NODE_AddStaticMeshComponent-0` :`RelativeTransform` (`KismetMathLibrary.MakeTransform` (`SplineComponent.GetLocationAtDistanceAlongSpline` (`self.Spline`) (* _index _distance) "Local")))))

(fn `UserConstructionScript`)